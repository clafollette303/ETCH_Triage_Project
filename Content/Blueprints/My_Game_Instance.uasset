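; Game instance for a pediatric triage training game, holding patient case data, player progress, the list of standing order sets and timer pause controls.
; SetCaseInfo fills a Cases map per patient with vitals, history, dialogue tree, sprites and correct answers.
; Setters record mistakes, ESI rating and chosen order by re-adding a copied struct, since map values cannot be edited in place.
; Final score sums dialogue accuracy plus rating and order bonuses over completed cases.
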(fn `AddScore`
  (params (ScoreToAdd :type Integer))
  ;[1 0.225 0.6933] Increments CurrentScore variable by value given.
  ; //NOTE: Scoring is calculated for each case, so this isn't used at the moment. I will save this for now.
  (set `self.CurrentScore` (+ ScoreToAdd (`self.CurrentScore`))))

(fn `CalculateCaseScore`
  (params (Case :type "/Game/Enums/CASE Enum (by ref)"))
  (returns (CaseScore :type Integer))
  (locals (Score :type Integer) (CaseDialogueOptions :type Integer) (ESIScore :type Integer))
  (bind _value (`BlueprintMapLibrary.Map_Find` (`self.Cases`) Case))
  ;[0.1012 0.5174 1] Set score = summation of all portions for case
  (bind _output_get (set `local.Score` (+ (`KismetMathLibrary.FTrunc` (* (/ (`KismetMathLibrary.Conv_IntToDouble` (break `/Game/Structs/Case_Info` _value)) (`KismetMathLibrary.Conv_IntToDouble` (+ (break `/Game/Structs/Case_Info` _value) (`.IncorrectDialogueOptions_16_7D61E89F465EC403457BAD9370946DA0` (break `/Game/Structs/Case_Info` _value))))) 1000.0)) (`local.Score`))))
  (`|ExecutionSequence`
    (:`then_0`
      (if (== (`.CorrectRating_8_A5ED9087424CEFE6C482C282EA4EF0EC` (break `/Game/Structs/Case_Info` _value)) (`.GivenRating_19_8F0A87B9460A2396FAAFBA9AC6CB0408` (break `/Game/Structs/Case_Info` _value)))
        (set `local.Score` (+ _output_get 500))))
    (:`then_1`
      (if (`KismetStringLibrary.EqualEqual_StrStr` (`.CorrectStandingOrder_11_364EB69E4C0C5CCD3B1C7D9A9D5CAF75` (break `/Game/Structs/Case_Info` _value)) (`.GivenStandingOrder_40_4CE0DDA0415D1D5E0933A08BC29F080D` (break `/Game/Structs/Case_Info` _value)))
        (set `local.Score` (+ _output_get 500)))
      (return _output_get))))

(fn `CalculateFinalScore`
  (returns (FinalScore :type Integer))
  (locals (Score :type Integer :default 0))
  ;[0.1292 0.4669 1] Calls CalculateScore for every case that has been completed, and returns the sum of those scores.
  (for _array_element (`self.CasesCompleted`)
    (bind _casescore (`self.CalculateCaseScore` _array_element))
    (set `local.Score` (+ _casescore (`local.Score`))))
  (return (`local.Score`)))

(fn `CaseCompleted`
  ;[0.1669 0.4103 1] Add a case when it is finished.
  (`KismetArrayLibrary.Array_Add` (`self.CasesCompleted`) (`self.CurrentCase`)))

(fn `GetCurrentScore`
  (returns (CurrentScore :type Integer))
  ;[1 0.2104 0.6179] Returns current score variable.
  ; //NOTE: Scoring is done for each case. This isn't used at the moment.
  (return (`self.CurrentScore`)))

(fn `GetStandingOrdersets`
  (returns (NewParam :type "Array of Text"))
  (return (`self.StandigOrdersets`)))

(fn `IncrementIncorrectDialogueOptions`
  (bind _value (`BlueprintMapLibrary.Map_Find` (`self.Cases`) (`self.CurrentCase`)))
  ;[0.07432 0.3973 1] Used to increment the number of incorrect dialogue options. Case needs to be completely copied otherwise the change will not be saved.
  (bind _result (`/Engine/EditorBlueprintResources/StandardMacros.IncrementInt` (`.IncorrectDialogueOptions_16_7D61E89F465EC403457BAD9370946DA0` (break `/Game/Structs/Case_Info` _value)))
    (:`  `
      (`BlueprintMapLibrary.Map_Add` (`self.Cases`) (`self.CurrentCase`) (make `/Game/Structs/Case_Info` (break `/Game/Structs/Case_Info` _value) _result (`.CorrectHotspots_5_7ADDE48E44B08EDEADD010AFFEC01CA8` (break `/Game/Structs/Case_Info` _value)) (`.IncorrectHotspotOptions_18_D45127D34312C0C5542F22B2E9266C8A` (break `/Game/Structs/Case_Info` _value)) (`.CorrectRating_8_A5ED9087424CEFE6C482C282EA4EF0EC` (break `/Game/Structs/Case_Info` _value)) (`.GivenRating_19_8F0A87B9460A2396FAAFBA9AC6CB0408` (break `/Game/Structs/Case_Info` _value)) (`.CorrectStandingOrder_11_364EB69E4C0C5CCD3B1C7D9A9D5CAF75` (break `/Game/Structs/Case_Info` _value)) (`.GivenStandingOrder_40_4CE0DDA0415D1D5E0933A08BC29F080D` (break `/Game/Structs/Case_Info` _value)) (`.PreAssess_24_2EEC736042202C49A92C14A4C4E35702` (break `/Game/Structs/Case_Info` _value)) (`.PastMedicalHistory_27_5395BD11407A17A2F31CE8BDC606458B` (break `/Game/Structs/Case_Info` _value)) (`.BeginCaseInfo_34_B8D55975478111422830DFA80F27549C` (break `/Game/Structs/Case_Info` _value)) (`.StartingTree_35_ED2689B44AC4682EE32E74A3CAFBBCD3` (break `/Game/Structs/Case_Info` _value)) (`.FrontSprite_44_9FF6D8E44A2FB82BABDA39817D1A2B53` (break `/Game/Structs/Case_Info` _value)) (`.SideSprtie_47_6DA023824C52C1A9F52B83A6818802B9` (break `/Game/Structs/Case_Info` _value)))))))

(fn `IncrementIncorrectHotspotOptions`
  (bind _value (`BlueprintMapLibrary.Map_Find` (`self.Cases`) (`self.CurrentCase`)))
  ;[1 0.3642 0.735] Deprecated for now. Hotspots are no longer correct or incorrect.
  (bind _result (`/Engine/EditorBlueprintResources/StandardMacros.IncrementInt` (`.IncorrectHotspotOptions_18_D45127D34312C0C5542F22B2E9266C8A` (break `/Game/Structs/Case_Info` _value)))
    (:`  `
      (`BlueprintMapLibrary.Map_Add` (`self.Cases`) (`self.CurrentCase`) (make `/Game/Structs/Case_Info` (break `/Game/Structs/Case_Info` _value) (`.IncorrectDialogueOptions_16_7D61E89F465EC403457BAD9370946DA0` (break `/Game/Structs/Case_Info` _value)) (`.CorrectHotspots_5_7ADDE48E44B08EDEADD010AFFEC01CA8` (break `/Game/Structs/Case_Info` _value)) _result (`.CorrectRating_8_A5ED9087424CEFE6C482C282EA4EF0EC` (break `/Game/Structs/Case_Info` _value)) (`.GivenRating_19_8F0A87B9460A2396FAAFBA9AC6CB0408` (break `/Game/Structs/Case_Info` _value)) (`.CorrectStandingOrder_11_364EB69E4C0C5CCD3B1C7D9A9D5CAF75` (break `/Game/Structs/Case_Info` _value)) (`.GivenStandingOrder_40_4CE0DDA0415D1D5E0933A08BC29F080D` (break `/Game/Structs/Case_Info` _value)) (`.PreAssess_24_2EEC736042202C49A92C14A4C4E35702` (break `/Game/Structs/Case_Info` _value)) (`.PastMedicalHistory_27_5395BD11407A17A2F31CE8BDC606458B` (break `/Game/Structs/Case_Info` _value)) (`.BeginCaseInfo_34_B8D55975478111422830DFA80F27549C` (break `/Game/Structs/Case_Info` _value)) (`.StartingTree_35_ED2689B44AC4682EE32E74A3CAFBBCD3` (break `/Game/Structs/Case_Info` _value)) (`.FrontSprite_44_9FF6D8E44A2FB82BABDA39817D1A2B53` (break `/Game/Structs/Case_Info` _value)) (`.SideSprtie_47_6DA023824C52C1A9F52B83A6818802B9` (break `/Game/Structs/Case_Info` _value)))))))

(fn `PauseTimer`
  (bind _timerprogressbar (`self.TimerProgressBar`))
  (bind _output_get (set `/Game/Widgets/W_Progress_Bar.IsStopped` true _timerprogressbar))
  (set `/Game/Widgets/W_Timer.IsStopped` _output_get (`/Game/Widgets/W_Progress_Bar.W_Timer` _timerprogressbar)))

(fn `ResumeTimer`
  (bind _timerprogressbar (`self.TimerProgressBar`))
  (bind _output_get (set `/Game/Widgets/W_Progress_Bar.IsStopped` false _timerprogressbar))
  (set `/Game/Widgets/W_Timer.IsStopped` _output_get (`/Game/Widgets/W_Progress_Bar.W_Timer` _timerprogressbar)))

(fn `SetCaseInfo`
  ;[0.116 0.3511 1] Switch case used to set the values of a specific case.
  ; This will probably look really super ugly once we have a bunch, but that's fine for now.
  (switch `/Game/Enums/CASE` (`self.CurrentCase`)
    (:`NewEnumerator0`
      (bind _output_get (set `self.CurrentCaseInfo` (make `/Game/Structs/Case_Info` 2 0 "LeftEar" 0 2 0 "Fever Management" "" "Weight: 16.3 kg \nHeart Rate: 167 BPM \nBlood Pressure: 103/61 \nTemperature: 103.1 ax \nO2: 98% RA \nRespiratory Rate: 30 \nLevel: ???" "" "Name: Jasmine \nAge: 8 years old \nComplaint: Left Ear Pain" "/Game/BehaviorTrees/Trees/CaseJasmine/BT_Dialogue_Jasmine.BT_Dialogue_Jasmine" "/Game/Sprites/SpriteJasmine.SpriteJasmine" "/Game/Sprites/SpriteJasmine.SpriteJasmine")))
      (`BlueprintMapLibrary.Map_Add` (`self.Cases`) (`self.CurrentCase`) _output_get))
    (:`NewEnumerator1`
      (bind _output_get_2 (set `self.CurrentCaseInfo` (make `/Game/Structs/Case_Info` 2 0 "" 0 2 0 "Vomiting" "" "Katie  \n10 yo \nF \nLevel 3 \nVomiting \nWeight: 35.2 kg \nHeart Rate: 133 BPM \nBlood Pressure: 111/67 \nTemperature: 97.8 oral \nO2: 99% RA \nRespiratory Rate: 38" "Patient Name: Katie  \n-History of asthma, adhd, and anxiety \n-Hospitalized for pneumonia October of 2023 \n-No known food or medication allergies \n-Home medications: Lexapro, methylphenidate,  \nflucasone inhaler, and albuterol as needed" "Name: Katie \nAge: 10 years old \nComplaint: Vomiting" "/Game/BehaviorTrees/Trees/CaseKatie/BT_Dialogue_Katie.BT_Dialogue_Katie" "/Game/Sprites/SpriteKatie.SpriteKatie" "/Game/Sprites/SpriteKatie.SpriteKatie")))
      (`BlueprintMapLibrary.Map_Add` (`self.Cases`) (`self.CurrentCase`) _output_get_2))))

(fn `SetGivenOrder`
  (params (GivenOrder :type Text))
  (bind _value (`BlueprintMapLibrary.Map_Find` (`self.Cases`) (`self.CurrentCase`)))
  (`BlueprintMapLibrary.Map_Add` (`self.Cases`) (`self.CurrentCase`) (make `/Game/Structs/Case_Info` (break `/Game/Structs/Case_Info` _value) (`.IncorrectDialogueOptions_16_7D61E89F465EC403457BAD9370946DA0` (break `/Game/Structs/Case_Info` _value)) (`.CorrectHotspots_5_7ADDE48E44B08EDEADD010AFFEC01CA8` (break `/Game/Structs/Case_Info` _value)) (`.IncorrectHotspotOptions_18_D45127D34312C0C5542F22B2E9266C8A` (break `/Game/Structs/Case_Info` _value)) (`.CorrectRating_8_A5ED9087424CEFE6C482C282EA4EF0EC` (break `/Game/Structs/Case_Info` _value)) (`.GivenRating_19_8F0A87B9460A2396FAAFBA9AC6CB0408` (break `/Game/Structs/Case_Info` _value)) (`.CorrectStandingOrder_11_364EB69E4C0C5CCD3B1C7D9A9D5CAF75` (break `/Game/Structs/Case_Info` _value)) (`KismetTextLibrary.Conv_TextToString` GivenOrder) (`.PreAssess_24_2EEC736042202C49A92C14A4C4E35702` (break `/Game/Structs/Case_Info` _value)) (`.PastMedicalHistory_27_5395BD11407A17A2F31CE8BDC606458B` (break `/Game/Structs/Case_Info` _value)) (`.BeginCaseInfo_34_B8D55975478111422830DFA80F27549C` (break `/Game/Structs/Case_Info` _value)) (`.StartingTree_35_ED2689B44AC4682EE32E74A3CAFBBCD3` (break `/Game/Structs/Case_Info` _value)) (`.FrontSprite_44_9FF6D8E44A2FB82BABDA39817D1A2B53` (break `/Game/Structs/Case_Info` _value)) (`.SideSprtie_47_6DA023824C52C1A9F52B83A6818802B9` (break `/Game/Structs/Case_Info` _value)))))

(fn `SetGivenRating`
  (params (GivenRating :type Integer))
  (bind _value (`BlueprintMapLibrary.Map_Find` (`self.Cases`) (`self.CurrentCase`)))
  ;[0.154 0.4642 1] Used to set the value of the ESI rating for this case. Case needs to be completely copied otherwise the change will not be saved.
  (`BlueprintMapLibrary.Map_Add` (`self.Cases`) (`self.CurrentCase`) (make `/Game/Structs/Case_Info` (break `/Game/Structs/Case_Info` _value) (`.IncorrectDialogueOptions_16_7D61E89F465EC403457BAD9370946DA0` (break `/Game/Structs/Case_Info` _value)) (`.CorrectHotspots_5_7ADDE48E44B08EDEADD010AFFEC01CA8` (break `/Game/Structs/Case_Info` _value)) (`.IncorrectHotspotOptions_18_D45127D34312C0C5542F22B2E9266C8A` (break `/Game/Structs/Case_Info` _value)) (`.CorrectRating_8_A5ED9087424CEFE6C482C282EA4EF0EC` (break `/Game/Structs/Case_Info` _value)) GivenRating (`.CorrectStandingOrder_11_364EB69E4C0C5CCD3B1C7D9A9D5CAF75` (break `/Game/Structs/Case_Info` _value)) (`.GivenStandingOrder_40_4CE0DDA0415D1D5E0933A08BC29F080D` (break `/Game/Structs/Case_Info` _value)) (`.PreAssess_24_2EEC736042202C49A92C14A4C4E35702` (break `/Game/Structs/Case_Info` _value)) (`.PastMedicalHistory_27_5395BD11407A17A2F31CE8BDC606458B` (break `/Game/Structs/Case_Info` _value)) (`.BeginCaseInfo_34_B8D55975478111422830DFA80F27549C` (break `/Game/Structs/Case_Info` _value)) (`.StartingTree_35_ED2689B44AC4682EE32E74A3CAFBBCD3` (break `/Game/Structs/Case_Info` _value)) (`.FrontSprite_44_9FF6D8E44A2FB82BABDA39817D1A2B53` (break `/Game/Structs/Case_Info` _value)) (`.SideSprtie_47_6DA023824C52C1A9F52B83A6818802B9` (break `/Game/Structs/Case_Info` _value)))))

(fn `SetPlayerDefaultCamera`
  ;[0.1707 0.5481 1] Resets the player based on current playerstart reference
  (`GameModeBase.RestartPlayerAtPlayerStart` (`GameplayStatics.GetGameMode`) (`GameplayStatics.GetPlayerController` 0) (`self.Player_Start`)))

(fn `SetPlayerStart`
  (params (PlayerStart :type "/Game/Blueprints/BP_Player_Start Object Reference"))
  ;[0.08689 0.4707 1] Set player start. Used when respawing the player to at the original camera POV.
  (set `self.Player_Start` PlayerStart))

(fn `SetStandingOrdersets`
  (set `self.StandigOrdersets` (`|MakeArray` "Abdominal Pain" "Asthma" "Behavioral Health" "Bladder Augmentation" "Chest Pain" "Epiglottitus" "Febrile Neonate" "Fever Management" "New Onset Diabetic DKA" "Pain in 6 mo or Older" "Shock" "Sickle Cell with Pain" "Stroke" "Suspected Sepsis" "Syncope" "Vomiting" "*Take Patient Stat to Trauma Room" :!type "Text")))