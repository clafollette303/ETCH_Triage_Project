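; Child pawn with a swappable Paper2D sprite that acts as a clickable entry point for behavior-tree-driven dialogue cases.
; Releasing a click on it hides the exclamation widget and starts the tree on BP_Child_Controller; Continue clears the running flag, fires CallContinue and reshows the widget.
; Helper functions spawn and remove screen-space widget components at runtime: dialogue buttons at preset offsets, which can also be disabled, and hotspots attached to sprite sockets.
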(event `self.ReceiveBeginPlay`
  ;[0.1312 0.4542 1] This is a list of locations for placing the dialogue buttons in the correct spots
  (bind _output_get (set `self.Vec3Location0` (-25.0 -120.0 196.0)))
  (bind _output_get_2 (set `self.Vec3Location1` (-100.0 99.0 157.0)))
  (bind _output_get_3 (set `self.Vec3Location2` (-50.0 61.0 196.0)))
  (bind _output_get_4 (set `self.Vec3Location3` (0.0 -50.0 125.0)))
  (set `self.ButtonLocations` (`|MakeArray` _output_get_4 _output_get_3 _output_get_2 _output_get))
  (bind _asw_exclaim_vfx (cast `/Game/Widgets/VFX_Anims/W_Exclaim_VFX` (`WidgetComponent.GetUserWidgetObject` (`self.ExclamationWidget`))))
  (add `/Game/Widgets/VFX_Anims/W_Exclaim_VFX.ImageClicked` _asw_exclaim_vfx (`|CreateDelegate` :!event `Event Start`)))

(event `self.ReceiveActorOnReleased`
  (params (ButtonReleased :type "Key Structure"))
  ;[0.1389 0.5027 1] Call start when clicked
  (`self.Event Start`))

(event `Event Start`
  ;[0.08993 0.4945 1] Starts dialogue tree
  (set `self.IsChildClicked` true)
  (`SceneComponent.SetVisibility` (`self.ExclamationWidget`) false false)
  (if (not (`self.TreeRunning`))
    (set `self.TreeRunning` true)
    (bind _asbp_child_controller (cast `/Game/Blueprints/Controllers/BP_Child_Controller` (`AIBlueprintHelperLibrary.GetAIController` self)))
    (set `/Game/Blueprints/Controllers/BP_Child_Controller.BehaviorTree` (`self.BehaviorTree`) _asbp_child_controller)
    (`/Game/Blueprints/Controllers/BP_Child_Controller.Start Behavior Tree` _asbp_child_controller)
    (set `self.IsChildClicked` false)))

(event `Event Continue`
  ;[0.1275 0.5156 1] Used to go from case to case.
  ; Also set tree running to false because this will only be called at the end of a case tree.
  (bind _output_get (set `self.TreeRunning` false))
  (set `/Game/Blueprints/Controllers/BP_Child_Controller.IsTreeRunning` _output_get (stale `Event Start` _asbp_child_controller))
  (`self.Continue`)
  (`SceneComponent.SetVisibility` (`self.ExclamationWidget`) true false))

(fn `AddButton`
  (params (ButtonToAdd :type "/Game/Widgets/Dialogue/W_Dialogue_Button Object Reference"))
  ;[0.1308 0.3481 1] Adds a button widget component to the child pawn based on the "ButtonLocations" array.
  (bind _returnvalue (`AddComponent|NODE_AddWidgetComponent-1` :`RelativeTransform` (`KismetMathLibrary.MakeTransform` (`|GetArrayItem` (`self.ButtonLocations`) (`self.ButtonIndex`)))))
  (`/Engine/EditorBlueprintResources/StandardMacros.IncrementInt` (`self.ButtonIndex`)
    (:`  `
      (`KismetArrayLibrary.Array_Add` (`self.ButtonComponents`) _returnvalue)
      (`WidgetComponent.SetWidget` _returnvalue ButtonToAdd)
      (`WidgetComponent.SetWidgetSpace` _returnvalue "Screen"))))

(fn `AddHotspot`
  (params (HotspotWidget :type "/Game/Widgets/VFX_Anims/W_Hotspot_VFX Object Reference") (Socket :type Name))
  ;[0.06918 0.5077 1] Adds a hotspot widget component to the child pawn based on the "HotspotLocations" array.
  ; Note that the array is not local to this class, but to the Case_Info struct based on the current case.
  (bind _returnvalue (`AddComponent|NODE_AddWidgetComponent-4`))
  (`SceneComponent.K2_AttachToComponent` _returnvalue (`self.PaperSprite`) Socket "KeepRelative" "KeepRelative" "KeepRelative" true)
  (`WidgetComponent.SetWidget` _returnvalue HotspotWidget)
  (`WidgetComponent.SetWidgetSpace` _returnvalue "Screen")
  (`KismetArrayLibrary.Array_Add` (`self.HotspotWidgets`) _returnvalue))

(fn `ClearButtons`
  ;[0.1292 0.4669 1] Clears dialogue buttons by destroying components that were added.
  ; Also resets the button index so that more can be added.
  (for _array_element (`self.ButtonComponents`)
    (`ActorComponent.K2_DestroyComponent` _array_element))
  (set `self.ButtonIndex` 0)
  (`KismetArrayLibrary.Array_Clear` (`self.ButtonComponents`)))

(fn `ClearHotspots`
  (bind _hotspotwidgets (`self.HotspotWidgets`))
  ;[0.08939 0.4583 1] Clears hotspots by destroying each of the components that were added.
  (for _array_element _hotspotwidgets
    (`ActorComponent.K2_DestroyComponent` _array_element))
  (`KismetArrayLibrary.Array_Clear` _hotspotwidgets))

(fn `DisableButtons`
  ;[0.0916 0.3821 1] Can be used to disable all buttons that were added in a dialogue section.
  (for _array_element (`self.ButtonComponents`)
    (`Widget.SetIsEnabled` (`WidgetComponent.GetUserWidgetObject` _array_element) false))
  (set `self.ButtonIndex` 0))

(fn `ResetLocation`
  (set `self.Vec3Location0` (100.0 75.0 205.0)))

(fn `SetSprite`
  (params (SpriteToSet :type "PaperSprite Object Reference (by ref)"))
  ;[0.07997 0.5303 1] Replaces the texture of child's sprite component
  (`PaperSpriteComponent.SetSprite` (`self.PaperSprite`) SpriteToSet))

(fn `UserConstructionScript`)